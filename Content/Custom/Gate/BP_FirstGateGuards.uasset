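; BP_FirstGateGuards tracks the guards of the first gate and moves that gate once all of them are destroyed.
; On BeginPlay it counts its child actors tagged Guard and caches the BP_Gate1 instance found in the level.
; A GuardDestroyed event decrements the count.
; Once started, Tick polls the count and, while it is zero, sets the gate to a hard-coded location every frame without interpolation.
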(event `self.ReceiveBeginPlay`
  (for _array_element (`self.GetAllChildActors` false)
    (if (`self.ActorHasTag` _array_element "Guard")
      (set `self.GuardCount` (+ (`self.GuardCount`) 1))))
  (bind _returnvalue (`GameplayStatics.GetActorOfClass` "/Game/Custom/Gate/BP_Gate1.BP_Gate1_C"))
  (set `self.Gate` _returnvalue)
  (set `self.Started` true))

(event `self.ReceiveTick`
  (params (DeltaSeconds :type "Float (single-precision)"))
  (if (`self.Started`)
    (if (== (`self.GuardCount`) 0)
      (`self.K2_SetActorLocation` (`self.Gate`) (1680.0 570.0 220.0) false false))))

(event `GuardDestroyed`
  (set `self.GuardCount` (- (`self.GuardCount`) 1)))

(fn `UserConstructionScript`)